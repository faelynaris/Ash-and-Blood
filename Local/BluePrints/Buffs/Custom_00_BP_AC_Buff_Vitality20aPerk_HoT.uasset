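; Heal-over-time buff component, apparently for the Vitality 20a perk, that sets the healing values on the owning player character.
; On begin play, buff start and timer reset, it spreads BuffPotency over BuffTicks, scales by PerkModifier and rounds up, cutting potency by a quarter if the owner has Vitality_10a.
; The result feeds both the initial boost and per-tick heal.
; The tooltip applies PerkModifier again to the per-tick value.
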(event EventBeginPlay
  (bind _buffpotency (Variables|Default|GetBuffPotency))
  (bind _perkmodifier (Variables|Default|GetPerkModifier))
  (bind _buffticks (Variables|Default|GetBuffTicks))
  (bind _returnvalue (Math|Conversions|ToFloat(Integer) _buffticks))
  (bind _returnvalue_2 (Math|Conversions|ToFloat(Integer) _buffpotency))
  (bind _asbase_player_char (Utilities|Casting|CastToBasePlayerChar (Components|GetOwner)))
  (if (Class|PerkSystemComponent|HasOwnedPerk (Variables|/Script/ConanSandbox.ConanCharacter|GetPerkSystemComponent _asbase_player_char) (Utilities|Name|MakeLiteralName "Vitality_10a"))
    (Variables|Default|SetHealingAmount (Math|Float|Ceil (* (/ (- _returnvalue_2 (* _returnvalue_2 0.25)) _returnvalue) _perkmodifier)))
    (else
      (Variables|Default|SetHealingAmount (Math|Float|Ceil (* (/ _returnvalue_2 _returnvalue) _perkmodifier)))))
  (Variables|Default|SetInitialHealthBoost (Variables|Default|GetHealingAmount))
  (Variables|Default|SetHealOverTimeValue (Variables|Default|GetHealingAmount)))

(event EventResetBuffTimer
  (bind _buffpotency (Variables|Default|GetBuffPotency))
  (bind _perkmodifier (Variables|Default|GetPerkModifier))
  (bind _buffticks (Variables|Default|GetBuffTicks))
  (bind _returnvalue (Math|Conversions|ToFloat(Integer) _buffticks))
  (bind _returnvalue_2 (Math|Conversions|ToFloat(Integer) _buffpotency))
  (bind _asbase_player_char (Utilities|Casting|CastToBasePlayerChar (Components|GetOwner)))
  (if (Class|PerkSystemComponent|HasOwnedPerk (Variables|/Script/ConanSandbox.ConanCharacter|GetPerkSystemComponent _asbase_player_char) (Utilities|Name|MakeLiteralName "Vitality_10a"))
    (Variables|Default|SetHealingAmount (Math|Float|Ceil (* (/ (- _returnvalue_2 (* _returnvalue_2 0.25)) _returnvalue) _perkmodifier)))
    (else
      (Variables|Default|SetHealingAmount (Math|Float|Ceil (* (/ _returnvalue_2 _returnvalue) _perkmodifier)))))
  (Variables|Default|SetInitialHealthBoost (Variables|Default|GetHealingAmount))
  (Variables|Default|SetHealOverTimeValue (Variables|Default|GetHealingAmount)))

(event EventGameplayEffecttoApplyonBuffStart
  (bind _buffpotency (Variables|Default|GetBuffPotency))
  (bind _perkmodifier (Variables|Default|GetPerkModifier))
  (bind _buffticks (Variables|Default|GetBuffTicks))
  (bind _returnvalue (Math|Conversions|ToFloat(Integer) _buffticks))
  (bind _returnvalue_2 (Math|Conversions|ToFloat(Integer) _buffpotency))
  (bind _asbase_player_char (Utilities|Casting|CastToBasePlayerChar (Components|GetOwner)))
  (if (Class|PerkSystemComponent|HasOwnedPerk (Variables|/Script/ConanSandbox.ConanCharacter|GetPerkSystemComponent _asbase_player_char) (Utilities|Name|MakeLiteralName "Vitality_10a"))
    (Variables|Default|SetHealingAmount (Math|Float|Ceil (* (/ (- _returnvalue_2 (* _returnvalue_2 0.25)) _returnvalue) _perkmodifier)))
    (else
      (Variables|Default|SetHealingAmount (Math|Float|Ceil (* (/ _returnvalue_2 _returnvalue) _perkmodifier)))))
  (Variables|Default|SetInitialHealthBoost (Variables|Default|GetHealingAmount))
  (Variables|Default|SetHealOverTimeValue (Variables|Default|GetHealingAmount)))

(fn GetEffectDescription
  (bind _bufftickduration (Variables|Default|GetBuffTickDuration))
  (bind _healovertimevalue (Variables|Default|GetHealOverTimeValue))
  (if (== _healovertimevalue 0)
    (return "")
    (else
      (return (Utilities|Text|FormatText "{TickDamage} points of healing every {TickTime}" (Math|Float|Truncate (* _healovertimevalue (Variables|Default|GetPerkModifier))) (select (> _bufftickduration 1.0) (Utilities|Text|FormatText "{TickTime} seconds" _bufftickduration) "second"))))))
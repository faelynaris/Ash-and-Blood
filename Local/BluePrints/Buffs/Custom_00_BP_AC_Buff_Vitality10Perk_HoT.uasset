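; Heal-over-time buff component for the Vitality 10 perk, which in this file only customizes its effect description text.
; GetEffectDescription returns an empty string when the heal value is zero, otherwise formats the heal value scaled by the perk modifier and truncated, along with the tick interval.
; The event graph holds only disabled placeholder events, so no healing logic appears here.
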(event EventBeginPlay)

(event EventTick
  (params (DeltaSeconds :type Float%20%28single-precision%29)))

(fn GetEffectDescription
  (bind _bufftickduration (Variables|Default|GetBuffTickDuration))
  (bind _healovertimevalue (Variables|Default|GetHealOverTimeValue))
  (if (== _healovertimevalue 0)
    (return "")
    (else
      (return (Utilities|Text|FormatText "{TickDamage} points of healing every {TickTime}" (Math|Float|Truncate (* _healovertimevalue (Variables|Default|GetPerkModifier))) (select (> _bufftickduration 1.0) (Utilities|Text|FormatText "{TickTime} seconds" _bufftickduration) "second"))))))
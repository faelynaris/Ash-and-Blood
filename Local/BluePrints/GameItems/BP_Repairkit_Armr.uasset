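; Armor repair kit item Blueprint that decides whether the kit can be dropped onto a target item.
; It accepts the drop only when the target's current durability is below its maximum after penalty loss and it is not already in a repair state.
; When durability leaves nothing to repair, it shows a cannot-drop notification for that item and rejects the drop.
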(fn CanbeDroppedonItem
  (params (TargetItem :type Game%20Item%20Object%20Reference))
  ;[1 1 1] Repairs are only allowed if the current durability is less than max durability after receiving durability penalty loss
  (LocalVariables|SetLocalItem TargetItem)
  (if (< (Class|GameItem|GetFloatStat (LocalVariables|GetLocalItem) "CurrentDurability") (CallFunction|GetMaxDurabilityAfterPenalty (LocalVariables|GetLocalItem)))
    (return (not (Class|GameItem|GetIsinRepairState (LocalVariables|GetLocalItem))))
    (else
      (CallFunction|ShowNotification (CallFunction|GetCannotDropReasonText "NewEnumerator11") (LocalVariables|GetLocalItem))
      (return false))))
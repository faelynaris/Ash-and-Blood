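; Armor repair kit inventory item that, when consumed on a target armor item, puts that armor into its repairing state.
; Drops are allowed only if the target's current durability is below its post-penalty maximum and it is not already being repaired.
; A target at or above that maximum rejects the drop and triggers a notification with the reason.
; The kit reports itself as neither armor nor projectile.
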(event EventOnConsumedfromInventory
  (params (Controller :type Conan%20Player%20Controller%20Object%20Reference) (TargetItem :type Game%20Item%20Object%20Reference))
  (bind _asbpgame_item_armor (Utilities|Casting|CastToBPGameItemArmor TargetItem))
  (Default|EnterRepairingState _asbpgame_item_armor 1.0))

(fn CanbeDroppedonItem
  (params (TargetItem :type Game%20Item%20Object%20Reference))
  (LocalVariables|SetLocalItem TargetItem)
  (if (< (Class|GameItem|GetFloatStat (LocalVariables|GetLocalItem) "CurrentDurability") (CallFunction|GetMaxDurabilityAfterPenalty (LocalVariables|GetLocalItem)))
    (return (not (Class|GameItem|GetIsinRepairState (LocalVariables|GetLocalItem))))
    (else
      (CallFunction|ShowNotification (CallFunction|GetCannotDropReasonText "NewEnumerator11") (LocalVariables|GetLocalItem))
      (return false))))

(fn IsArmour
  (return false))

(fn IsProjectile
  (return false))
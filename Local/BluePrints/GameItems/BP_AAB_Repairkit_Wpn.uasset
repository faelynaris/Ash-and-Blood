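; Weapon repair kit item that is dropped onto a weapon in the inventory to repair it.
; The drop check rejects items already repairing, rune-enchanted ones found via the modkit table, three excluded template IDs, and those not below penalty-adjusted max durability, with notifications for most refusals.
; On consumption it updates the RepairWeapon journey event and puts the target weapon into its repairing state.
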(event EventOnConsumedfromInventory
  (params (Controller :type Conan%20Player%20Controller%20Object%20Reference) (TargetItem :type Game%20Item%20Object%20Reference))
  (bind _asbpgame_item_weapon (Utilities|Casting|CastToBPGameItemWeapon TargetItem))
  (Default|UpdateJourneyEvent _asbpgame_item_weapon Controller "RepairWeapon")
  (Default|EnterRepairingState _asbpgame_item_weapon 1.0))

(fn CanbeDroppedonItem
  (params (TargetItem :type Game%20Item%20Object%20Reference))
  (LocalVariables|SetLocalItem TargetItem)
  (if (Class|GameItem|GetIsinRepairState (LocalVariables|GetLocalItem))
    (return false)
    (else
      (if (!= (Class|GameItem|GetIntStat (LocalVariables|GetLocalItem) "CurrentEnchantID") 0)
        ;[1 1 1] Cannot repair items that are rune-enchanted
        (bind _returnvalue (Utilities|GetDataTableRow "/Game/Systems/RiddleOfSteel/WeaponModkitTable.WeaponModkitTable" (Utilities|String|StringToName (Utilities|String|ToString(Integer) (Class|GameItem|GetIntStat (LocalVariables|GetLocalItem) "CurrentEnchantID"))))
          (:then
            (if (.IsARune (Utilities|Struct|BreakWeaponModkitTableRow _returnvalue))
              (CallFunction|ShowNotification (CallFunction|GetCannotDropReasonText "NewEnumerator6") (LocalVariables|GetLocalItem))
              (return false)
              (else
                _)))
          (:RowNotFound
            _)))
      (if (Math|Boolean|ANDBoolean (not (== (Variables|/Script/ConanSandbox.GameItem|GetTemplateID (LocalVariables|GetLocalItem)) 51468)) (not (== (Variables|/Script/ConanSandbox.GameItem|GetTemplateID (LocalVariables|GetLocalItem)) 51545)) (not (== (Variables|/Script/ConanSandbox.GameItem|GetTemplateID (LocalVariables|GetLocalItem)) 50592)))
        (if (< (Class|GameItem|GetFloatStat (LocalVariables|GetLocalItem) "CurrentDurability") (CallFunction|GetMaxDurabilityAfterPenalty (LocalVariables|GetLocalItem)))
          (return true)
          (else
            (CallFunction|ShowNotification (CallFunction|GetCannotDropReasonText "NewEnumerator8") (LocalVariables|GetLocalItem))
            (return false)))
        (else
          (CallFunction|ShowNotification (CallFunction|GetCannotDropReasonText "NewEnumerator6") (LocalVariables|GetLocalItem))
          (return false))))))

(fn IsArmour
  (return false))

(fn IsProjectile
  (return false))
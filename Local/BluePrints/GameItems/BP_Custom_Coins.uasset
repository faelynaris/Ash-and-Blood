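; BP_Custom_Coins is a coin item Blueprint that controls where coins can be moved between inventories.
; AllowsMoveTo permits moves within the owner's inventory and blocks moves into other inventories owned by a BP_LootContainer.
; Targets whose owner's display name contains the trader NPC substring are allowed before that container cast runs, and all other targets are allowed too.
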(fn AllowsMoveto
  (params (srcIndex :type Integer) (targetInventory :type Item%20Inventory%20Object%20Reference) (targetIndex :type Integer) (quantity :type Integer))
  (bind _returnvalue (Components|GetOwner targetInventory))
  (if (== targetInventory (Class|GameItem|GetOwnerInventory))
    (return true)
    (else
      (if (Utilities|String|Contains (Utilities|GetDisplayName _returnvalue) "tot_a_tradernpc")
        _
        (else
          (Utilities|Casting|CastToBP_LootContainer _returnvalue
            (:then
              (return false))
            (:CastFailed
              _))))
      (return true))))
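; Actor component for BP_PL_Crafting_Station that grants thrall-based bonus recipes and stat bonuses on crafted items.
; The active thrall's profession row sets the station's artisan tier, profession and recipe inventory.
; For benches in DT_CustomBenchIDs, queue events maintain parallel arrays pairing each queued recipe with its thrall bonus row.
; On crafting, the first queued entry's row applies int and float stat multipliers to weapons, armor and tools.
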(event Custom|Update%20Bonus%20Recipe%20LIst
  (params (New%20Active%20Thrall :type Name) (New%20Active%20Thrall%20Bonus%20Row :type Name) (Thrall%20Profession :type Name))
  (Variables|Default|SetNew%20Active%20Thrall New%20Active%20Thrall)
  (Variables|Default|SetNew%20Active%20Thrall%20Bonus%20Row New%20Active%20Thrall%20Bonus%20Row)
  (Variables|Default|SetThrall%20Profession Thrall%20Profession)
  (CallFunction|UpdateRecipeList))

(event Custom|OnQueEmpty
  (params (craftingQueue :type Crafting%20Queue%20Object%20Reference))
  (Utilities|Array|Clear (Variables|Default|GetCrafted%20Recipes))
  (Utilities|Array|Clear (Variables|Default|GetThrall%20Used))
  (Development|PrintString "Que is empty"))

(event Custom|OnRecipeCancelled
  (params (index :type Integer) (item :type Game%20Item%20Object%20Reference) (dstInventory :type Item%20Inventory%20Object%20Reference) (dstIndex :type Integer))
  (bind _crafted_recipes (Variables|Default|GetCrafted%20Recipes))
  (bind _thrall_used (Variables|Default|GetThrall%20Used))
  (Utilities|FlowControl|Delay 0.2)
  (if (== (Class|GameItem|GetIntStat item "StackSize") 1)
    (if (Variables|Default|Getwas%20Item%20Crafted)
      (Utilities|Array|RemoveIndex _crafted_recipes)
      (Utilities|Array|RemoveIndex _thrall_used)
      (Variables|Default|Setwas%20Item%20Crafted false)
      (Development|PrintString (Utilities|String|ToString(Text) (Utilities|Text|FormatText "Recipe removed at index [0]")))
      (else
        (Utilities|Array|RemoveIndex _crafted_recipes index)
        (Utilities|Array|RemoveIndex _thrall_used index)
        (Development|PrintString (Utilities|String|ToString(Text) (Utilities|Text|FormatText "Recipe removed at index [{index}]" index)))))))

(event Custom|OnItemAddedToQue
  (params (index :type Integer) (item :type Game%20Item%20Object%20Reference) (srcInventory :type Item%20Inventory%20Object%20Reference) (srcIndex :type Integer))
  (bind _new_active_thrall_bonus_row (Variables|Default|GetNew%20Active%20Thrall%20Bonus%20Row))
  (bind _returnvalue (Class|GameItemSpawner|SpawnRecipeItem (Variables|/Script/ConanSandbox.GameItem|GetTemplateID item)))
  (Utilities|Array|Add (Variables|Default|GetCrafted%20Recipes) _returnvalue)
  (Utilities|Array|Add (Variables|Default|GetThrall%20Used) _new_active_thrall_bonus_row)
  (Development|PrintString (Utilities|String|ToString(Text) (Utilities|Text|FormatText "Recipe added with Thrall Bonus [{bonus}]" (Utilities|Text|ToText(String) (Utilities|String|ToString(Name) _new_active_thrall_bonus_row))))))

(event Custom|CraftingSystem%20OnItemCrafted
  (bind _crafting_station (Variables|Default|GetCrafting%20Station))
  (bind _craftingqueue (Variables|/Game/Systems/Building/Placeables/BP_PL_Crafting_Station.BP_PL_Crafting_Station_C|GetCraftingQueue _crafting_station))
  (Utilities|GetDataTableRow "/Game/Mods/Ash-and-Blood/DataTables/DefaultTables/DT_CustomBenchIDs.DT_CustomBenchIDs" (Utilities|String|StringToName (Utilities|String|ToString(Integer) (Variables|/Script/ConanSandbox.BuildableBase|GetTemplateId _crafting_station)))
    (:then
      (Utilities|FlowControl|Sequence
        (:then_0
          (EventDispatchers|BindEventtoSignalItemCrafted _craftingqueue (delegate Custom|OnItemCrafted)))
        (:then_1
          (EventDispatchers|BindEventtoSignalItemAdded _craftingqueue (delegate Custom|OnItemAddedToQue)))
        (:then_2
          (EventDispatchers|BindEventtoSignalItemRemoved _craftingqueue (delegate Custom|OnRecipeCancelled)))
        (:then_3
          (EventDispatchers|BindEventtoSignalQueueEmpty _craftingqueue (delegate Custom|OnQueEmpty)))))))

(event Custom|OnItemCrafted
  (params (recipeItem :type Recipe%20Item%20Object%20Reference) (gameItem :type Game%20Item%20Object%20Reference) (stackSize :type Integer))
  (bind _thrall_used (Variables|Default|GetThrall%20Used))
  (bind _crafting_station (Variables|Default|GetCrafting%20Station))
  (bind _item (Utilities|Array|Get(acopy) _thrall_used))
  (if (Utilities|Enum|Equal(Enum) (Class|GameItem|GetItemName recipeItem) (Class|GameItem|GetItemName (Utilities|Array|Get(acopy) (Variables|Default|GetCrafted%20Recipes))))
    (bind _output_get (Variables|Default|SetTemp%20Game%20Item%20Crafted gameItem))
    (switch Utilities|FlowControl|Switch|SwitchonEGameItemGUICategory (Class|GameItem|GetGUICategory _output_get)
      (:Weapon
        _)
      (:Armor
        _)
      (:Tools
        _))
    (Utilities|IsValid _output_get
      (:Is%20Valid
        (bind _returnvalue (Utilities|GetDataTableRow "/Game/Systems/Crafting/DT_ThrallItemCraftBonuses.DT_ThrallItemCraftBonuses" _item)
          (:then
            (for _array_element (.TierBonuses (Utilities|Struct|BreakSTR_ThrallCraftingProfessionToBonusesMapping _returnvalue))
              (for (_array_element_2 _array_index) (.IntStats (Utilities|Struct|BreakSTR_ThrallCraftingItemStatBonuses (.Bonuses (Utilities|Struct|BreakSTR_ThrallTiersSubstruct _array_element))))
                (Default|SetIntStatBonuses _crafting_station _array_element_2 (Utilities|Array|Get(acopy) (.IntStats_Bonuses (Utilities|Struct|BreakSTR_ThrallCraftingItemStatBonuses (.Bonuses (Utilities|Struct|BreakSTR_ThrallTiersSubstruct _array_element)))) _array_index) (Variables|Default|GetTemp%20Game%20Item%20Crafted)))
              (for (_array_element_3 _array_index_2) (.FloatStats (Utilities|Struct|BreakSTR_ThrallCraftingItemStatBonuses (.Bonuses (Utilities|Struct|BreakSTR_ThrallTiersSubstruct _array_element))))
                (Default|SetFloatStatBonuses _crafting_station _array_element_3 (Utilities|Array|Get(acopy) (.FloatStats_Bonuses (Utilities|Struct|BreakSTR_ThrallCraftingItemStatBonuses (.Bonuses (Utilities|Struct|BreakSTR_ThrallTiersSubstruct _array_element)))) _array_index_2) (Variables|Default|GetTemp%20Game%20Item%20Crafted))))
            (Variables|Default|Setwas%20Item%20Crafted true)
            (Development|PrintString (Utilities|String|ToString(Text) (Utilities|Text|FormatText "Item upgraded at [{index}]" (Utilities|Text|ToText(String) (Utilities|String|ToString(Name) _item)))) true true "(R=0.000000,G=0.660000,B=1.000000,A=1.000000)" 5.0)))))
    (else
      (Variables|Default|Setwas%20Item%20Crafted true)
      (Development|PrintString "Recipe Not Found."))))

(event Custom|Multicast%20Update%20Recipes
  (CallFunction|UpdateRecipeList))

(event EventBeginPlay
  (Utilities|FlowControl|Delay 0.25)
  (bind _asbp_pl_crafting_station (Utilities|Casting|CastToBP_PL_Crafting_Station (Components|GetOwner)))
  (Variables|Default|SetCrafting%20Station _asbp_pl_crafting_station)
  (CallFunction|CraftingSystemonItemCrafted)
  (CallFunction|MulticastUpdateRecipes))

(fn UpdateRecipeList
  (bind _crafting_station (Variables|Default|GetCrafting%20Station))
  (bind _crafting_station_2 (Variables|Default|GetCrafting%20Station))
  (bind _new_recipe_inventory (Variables|Default|GetNew%20Recipe%20Inventory))
  (bind _crafting_station_3 (Variables|Default|GetCrafting%20Station))
  (bind _conanbuildingpersistence (Variables|/Game/Systems/Building/Placeables/BP_Master_Placeables.BP_Master_Placeables_C|GetConanBuildingPersistence _crafting_station))
  (bind _returnvalue (Utilities|GetDataTableRow "/Game/Systems/SpawnTable/ProfessionTemplateDataTable.ProfessionTemplateDataTable" (Variables|Default|GetThrall%20Profession))
    (:then
      (Utilities|Array|Clear _new_recipe_inventory)
      (Variables|/Game/Systems/Building/Placeables/BP_PL_Crafting_Station.BP_PL_Crafting_Station_C|SetCurrentArtisanTier _crafting_station_2 (.ThrallTier (Utilities|Struct|BreakProfessionTemplateTableRow _returnvalue)))
      (Variables|/Game/Systems/Building/Placeables/BP_PL_Crafting_Station.BP_PL_Crafting_Station_C|SetCurrentArtisanProfession _crafting_station_3 (.ThrallProfession (Utilities|Struct|BreakProfessionTemplateTableRow _returnvalue)))
      (for _array_element (.BonusRecipes (Utilities|Struct|BreakProfessionTemplateTableRow _returnvalue))
        (bind _returnvalue_2 (Class|GameItemSpawner|SpawnItem "Recipe" _array_element))
        (Utilities|Array|Add (Variables|Default|GetNew%20Recipe%20Inventory) _returnvalue_2))
      (Variables|/Script/ConanSandbox.ItemInventory|SetItemList (Variables|/Game/Systems/Building/Placeables/BP_PL_Crafting_Station.BP_PL_Crafting_Station_C|GetArtisanRecipeInventory _crafting_station) (Variables|Default|GetNew%20Recipe%20Inventory))
      (Variables|/Game/Systems/Building/Placeables/BP_PL_Crafting_Station.BP_PL_Crafting_Station_C|SetArtisanRecipeInventory _crafting_station (Variables|/Game/Systems/Building/Placeables/BP_PL_Crafting_Station.BP_PL_Crafting_Station_C|GetArtisanRecipeInventory _crafting_station))
      (Utilities|IsValid _conanbuildingpersistence
        (:Is%20Valid
          (Class|PersistenceComponent|SetDirty _conanbuildingpersistence true 5.0))))
    (:RowNotFound
      (Utilities|Array|Clear _new_recipe_inventory)
      (Variables|/Game/Systems/Building/Placeables/BP_PL_Crafting_Station.BP_PL_Crafting_Station_C|SetCurrentArtisanTier _crafting_station_2 0)
      (Variables|/Game/Systems/Building/Placeables/BP_PL_Crafting_Station.BP_PL_Crafting_Station_C|SetCurrentArtisanProfession _crafting_station_3 "Performer"))))
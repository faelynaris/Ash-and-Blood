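; Actor component that gives placeable chest containers bulk material storage, tallying items other than weapons, armor and consumables outside the normal inventory.
; After a short BeginPlay delay, it sets non-brush containers' item limit from MC_AnB by template ID.
; Existing and newly added materials are summed into parallel template-ID and amount arrays, then deleted from the inventory (server-only for new additions).
; Non-server instances push updated totals to the crafting GUI, and RemoveItemsFromStorage decrements them.
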(event Custom|OnItemAddedToInventory
  (params (index :type Integer) (item :type Game%20Item%20Object%20Reference) (srcInventory :type Item%20Inventory%20Object%20Reference) (srcIndex :type Integer))
  (Variables|Default|SetStored%20Item item)
  (if (not (Math|Boolean|ORBoolean (Utilities|Enum|Equal(Enum) (Class|GameItem|GetGUICategory (Variables|Default|GetStored%20Item)) "Weapon") (Utilities|Enum|Equal(Enum) (Class|GameItem|GetGUICategory (Variables|Default|GetStored%20Item)) "Armor") (Utilities|Enum|Equal(Enum) (Class|GameItem|GetGUICategory (Variables|Default|GetStored%20Item)) "Consumable")))
    (if (!= (Utilities|Array|FindItem (Variables|Default|GetStorage-%20Template%20ID) (Variables|/Script/ConanSandbox.GameItem|GetTemplateID (Variables|Default|GetStored%20Item))) -1)
      (Utilities|Array|SetArrayElem (Variables|Default|GetStorage-%20Amounts) (Utilities|Array|FindItem (Variables|Default|GetStorage-%20Template%20ID) (Variables|/Script/ConanSandbox.GameItem|GetTemplateID (Variables|Default|GetStored%20Item))) (+ (Utilities|Array|Get(acopy) (Variables|Default|GetStorage-%20Amounts) (Utilities|Array|FindItem (Variables|Default|GetStorage-%20Template%20ID) (Variables|/Script/ConanSandbox.GameItem|GetTemplateID (Variables|Default|GetStored%20Item)))) (Class|GameItem|GetIntStat (Variables|Default|GetStored%20Item) "StackSize")))
      (Utilities|FlowControl|Delay 0.25)
      (else
        (Utilities|Array|Add (Variables|Default|GetStorage-%20Template%20ID) (Variables|/Script/ConanSandbox.GameItem|GetTemplateID (Variables|Default|GetStored%20Item)))
        (Utilities|Array|Add (Variables|Default|GetStorage-%20Amounts) (Class|GameItem|GetIntStat (Variables|Default|GetStored%20Item) "StackSize"))))
    (if (not (Networking|IsServer))
      (bind _foundwidgets (Widget|GetAllWidgetsOfClass "/Game/Mods/Ash-and-Blood/UserInterface/W_AAB_CraftingGUI.W_AAB_CraftingGUI_C" true))
      (Utilities|IsValid (Utilities|Array|Get(acopy) _foundwidgets)
        (:Is%20Valid
          (Default|UpdateInventory (Utilities|Array|Get(acopy) _foundwidgets) (Variables|Default|GetStorage-%20Template%20ID) (Variables|Default|GetStorage-%20Amounts))))
      (else
        (bind _returnvalue (Class|ItemInventory|DeleteItemsbyTemplate (Variables|/Game/Systems/Building/Placeables/BP_PlaceableItemContainer.BP_PlaceableItemContainer_C|GetPlaceableInventory (Variables|Default|GetPlaceableItemContainer)) (Variables|/Script/ConanSandbox.GameItem|GetTemplateID (Variables|Default|GetStored%20Item)) "None" (Class|GameItem|GetIntStat (Variables|Default|GetStored%20Item) "StackSize")))
        (Development|PrintString (Utilities|String|ToString(Text) (Utilities|Text|FormatText "Items Stored.
Items deleted == {bool}" (select _returnvalue "T" "F"))))))))

(event Custom|MaterialStorageInventorySystem_Activate
  (EventDispatchers|BindEventtoSignalItemAdded (Actor|GetComponentbyClass (Variables|Default|GetPlaceableItemContainer) "/Script/ConanSandbox.ItemInventoryReplicateToAll") (delegate Custom|OnItemAddedToInventory))
  (CallFunction|InitialSetupOfStorage))

(event EventBeginPlay
  (Utilities|FlowControl|Delay 0.25)
  (bind _asbp_placeable_item_container (Utilities|Casting|CastToBP_PlaceableItemContainer (Components|GetOwner)))
  (Variables|Default|SetPlaceableItemContainer _asbp_placeable_item_container)
  (CallFunction|CalculateStorage)
  (CallFunction|MaterialStorageInventorySystemActivate))

(fn CalculateStorage
  (bind _placeableitemcontainer (Variables|Default|GetPlaceableItemContainer))
  (bind _returnvalue (Actor|GetComponentbyClass _placeableitemcontainer "/Script/ConanSandbox.ItemInventoryReplicateToAll"))
  (bind _templateid (Variables|/Script/ConanSandbox.BuildableBase|GetTemplateId _placeableitemcontainer))
  (bind _outactors (Actor|GetAllActorsOfClass "/Game/Mods/Ash-and-Blood/MC_AnB.MC_AnB_C"))
  (if (not (Variables|/Script/ConanSandbox.BuildableBase|GetIsABrush _placeableitemcontainer))
    (if (== (Utilities|Array|FindItem (Variables|/Game/Mods/Ash-and-Blood/MC_AnB.MC_AnB_C|GetLimitations%20-%20Storage%20Containers%20IDs (Utilities|Array|Get(acopy) _outactors)) _templateid) -1)
      (Variables|Default|SetStorage%20Amount 0)
      (else
        (Variables|Default|SetStorage%20Amount (Default|GetStorageAmountfromTemplateID (Utilities|Array|Get(acopy) _outactors) _templateid))))
    (if (Utilities|IsValid _returnvalue)
      (Class|ItemInventory|SetMaxItemCount _returnvalue (Variables|Default|GetStorage%20Amount)))))

(fn RemoveItemsfromStorage
  (params (Index :type Integer) (Amount :type Integer))
  (bind _storage__amounts (Variables|Default|GetStorage-%20Amounts))
  (bind _item (Utilities|Array|Get(acopy) _storage__amounts Index))
  (Utilities|Array|SetArrayElem _storage__amounts Index (- _item Amount))
  (if (== _item 0)
    (Utilities|Array|RemoveIndex (Variables|Default|GetStorage-%20Amounts) Index)
    (Utilities|Array|RemoveIndex (Variables|Default|GetStorage-%20Template%20ID) Index)))

(fn InitialSetupOfStorage
  (bind _placeableitemcontainer (Variables|Default|GetPlaceableItemContainer))
  (bind _placeableitemcontainer_2 (Variables|Default|GetPlaceableItemContainer))
  (bind _placeableinventory (Variables|/Game/Systems/Building/Placeables/BP_PlaceableItemContainer.BP_PlaceableItemContainer_C|GetPlaceableInventory _placeableitemcontainer))
  (bind _placeableinventory_2 (Variables|/Game/Systems/Building/Placeables/BP_PlaceableItemContainer.BP_PlaceableItemContainer_C|GetPlaceableInventory _placeableitemcontainer_2))
  (bind _itemlist (Variables|/Script/ConanSandbox.ItemInventory|GetItemList _placeableinventory))
  (if (> (Utilities|Array|Length _itemlist) 0)
    (for _array_element _itemlist
      (Variables|Default|SetStored%20Item _array_element)
      (if (not (Math|Boolean|ORBoolean (Utilities|Enum|Equal(Enum) (Class|GameItem|GetGUICategory (Variables|Default|GetStored%20Item)) "Weapon") (Utilities|Enum|Equal(Enum) (Class|GameItem|GetGUICategory (Variables|Default|GetStored%20Item)) "Armor") (Utilities|Enum|Equal(Enum) (Class|GameItem|GetGUICategory (Variables|Default|GetStored%20Item)) "Consumable")))
        (if (!= (Utilities|Array|FindItem (Variables|Default|GetStorage-%20Template%20ID) (Variables|/Script/ConanSandbox.GameItem|GetTemplateID (Variables|Default|GetStored%20Item))) -1)
          (Utilities|Array|SetArrayElem (Variables|Default|GetStorage-%20Amounts) (Utilities|Array|FindItem (Variables|Default|GetStorage-%20Template%20ID) (Variables|/Script/ConanSandbox.GameItem|GetTemplateID (Variables|Default|GetStored%20Item))) (+ (Utilities|Array|Get(acopy) (Variables|Default|GetStorage-%20Amounts) (Utilities|Array|FindItem (Variables|Default|GetStorage-%20Template%20ID) (Variables|/Script/ConanSandbox.GameItem|GetTemplateID (Variables|Default|GetStored%20Item)))) (Class|GameItem|GetIntStat (Variables|Default|GetStored%20Item) "StackSize")))
          (else
            (Utilities|Array|Add (Variables|Default|GetStorage-%20Template%20ID) (Variables|/Script/ConanSandbox.GameItem|GetTemplateID (Variables|Default|GetStored%20Item)))
            (Utilities|Array|Add (Variables|Default|GetStorage-%20Amounts) (Class|GameItem|GetIntStat (Variables|Default|GetStored%20Item) "StackSize"))))
        (Class|ItemInventory|DeleteItems _placeableinventory_2 (Class|ItemInventory|GetItemIndex _placeableinventory_2 (Variables|Default|GetStored%20Item)) "None" (Class|GameItem|GetIntStat (Variables|Default|GetStored%20Item) "StackSize"))))))
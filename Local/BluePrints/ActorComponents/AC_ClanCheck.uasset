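; Actor component that blocks player characters without a clan from using construction tools.
; On BeginPlay it casts its owner to BasePlayerChar and binds to that player's weapon-equipped signal.
; When the equipped item is a BPGameItemConstructionTool and the player has no valid guild, it unequips weapons and shows a HUD notification saying a clan is required to build.
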(event Custom|NotHammerTime
  (params (Item :type Game%20Item%20Object%20Reference))
  (Utilities|Casting|CastToBPGameItemConstructionTool Item)
  (if (not (Utilities|IsValid (Class|ConanCharacter|GetGuild (Variables|Default|GetPlayer))))
    (Default|UnequipWeapons (Variables|Default|GetPlayer))
    (Class|ConanCharacter|ClientHUDShowNotification (Variables|Default|GetPlayer) (Utilities|Text|MakeLiteralText "You can not build without being part of a clan. Please create one, even if you are solo.") true true)))

(event EventBeginPlay
  (bind _asbase_player_char (Utilities|Casting|CastToBasePlayerChar (Components|GetOwner)))
  (bind _output_get (Variables|Default|SetPlayer _asbase_player_char))
  (EventDispatchers|BindEventtoSignalWeaponEquipped _output_get (delegate Custom|NotHammerTime)))

(event EventTick
  (params (DeltaSeconds :type Float%20%28single-precision%29)))
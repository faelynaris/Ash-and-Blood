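; Player character component for custom mod rules: swaps the Vitality perk heal-over-time buff for a custom one on damage.
; It records interacted crafting stations and loot containers, and relays item takes and thrall crafting bonuses through Server events.
; It totals owned storage usage plus guild role bonuses, toggling a RepNotify to refresh the guild UI.
; A DataTable-driven potion cap returns excess items to their source, but its setup is disconnected from BeginPlay.
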(event EventBeginPlay
  (bind _asbase_player_char (Utilities|Casting|CastToBasePlayerChar (Components|GetOwner)))
  (Variables|Default|SetBasePlayerChar _asbase_player_char)
  (bind _outactors (Actor|GetAllActorsOfClass "/Game/Mods/Ash-and-Blood/MC_AnB.MC_AnB_C"))
  (Variables|Default|SetModController (Utilities|Array|Get(acopy) _outactors))
  (CallFunction|RunReplaceGluttonBluff)
  (CallFunction|CustomInteractableActivate))

(event Custom|OnInteractPressed
  ;[0 1 0.06933] Custom Interactable Activate
  (Utilities|IsInterfaceValid? (Variables|/Game/Systems/InteractionManager.InteractionManager_C|GetSelectedObject (Default|GetInteractionManager (stale Custom|Custom%20Interactable%20Activate _asfun_combat_player_controller)))
    (:IsValid
      (bind _asbp_placeable_item_container (Utilities|Casting|CastToBP_PlaceableItemContainer (Variables|/Game/Systems/InteractionManager.InteractionManager_C|GetSelectedObject (Default|GetInteractionManager (stale Custom|Custom%20Interactable%20Activate _asfun_combat_player_controller))))
        (:then
          (bind _asbp_pl_crafting_station (Utilities|Casting|CastToBP_PL_Crafting_Station (Variables|/Game/Systems/InteractionManager.InteractionManager_C|GetSelectedObject (Default|GetInteractionManager (stale Custom|Custom%20Interactable%20Activate _asfun_combat_player_controller)))))
          (CallFunction|ServerSetInteractedCraftingStation _asbp_pl_crafting_station))
        (:CastFailed
          (bind _asbp_loot_container (Utilities|Casting|CastToBP_LootContainer (Variables|/Game/Systems/InteractionManager.InteractionManager_C|GetSelectedObject (Default|GetInteractionManager (stale Custom|Custom%20Interactable%20Activate _asfun_combat_player_controller)))))
          (CallFunction|ServerSetInteractedLootContainer _asbp_loot_container))))))

(event Custom|Run%20Replace%20Glutton%20Bluff
  (EventDispatchers|BindEventtoOnTakeAnyDamage (Variables|Default|GetBasePlayerChar) (delegate Custom|CustomOnTakeAnyDamage)))

(event Custom|Server%20Take%20Items
  (params (Item%20Container :type BP%20Placeable%20Item%20Container%20Object%20Reference) (Index :type Integer) (Take%20Amount :type Integer))
  (bind _returnvalue (Actor|GetComponentbyClass Item%20Container "/Game/Mods/Ash-and-Blood/BluePrints/ActorComponents/AC_ChestStorageEnabled.AC_ChestStorageEnabled_C"))
  (Class|ItemInventory|AddItemTemplate (Variables|/Game/Characters/BasePlayerChar.BasePlayerChar_C|GetBackpackInventory (Variables|Default|GetBasePlayerChar)) (Utilities|Array|Get(acopy) (Variables|/Game/Mods/Ash-and-Blood/BluePrints/ActorComponents/AC_ChestStorageEnabled.AC_ChestStorageEnabled_C|GetStorage-%20Template%20ID _returnvalue) Index) -1 "None" Take%20Amount false 1.0 -1.0)
  (Default|RemoveItemsfromStorage _returnvalue Index Take%20Amount))

(event Custom|Restrict%20Specific%20Items%20by%20Amount%20IntStatChange
  (EventDispatchers|BindEventtoSignalItemIntStatChanged (Variables|Default|GetBackpack%20Inventory) (delegate Custom|OnIntStatChangedBackpack))
  (EventDispatchers|BindEventtoSignalItemIntStatChanged (Variables|Default|GetShortcutBar%20Inventory) (delegate Custom|OnIntStatChangedShortcutBar)))

(event Custom|OnIntStatChangedBackpack
  (params (item :type Game%20Item%20Object%20Reference) (statID :type EItemIntStatID%20Enum) (statValue :type Integer) (deltaValue :type Integer))
  (bind _interactedstoragecontainer (Variables|Default|GetInteractedStorageContainer))
  (bind _interacted_loot_container (Variables|Default|GetInteracted%20Loot%20Container))
  (bind _placeableinventory (Variables|/Game/Systems/Building/Placeables/BP_PlaceableItemContainer.BP_PlaceableItemContainer_C|GetPlaceableInventory _interactedstoragecontainer))
  (bind _iteminventory (Variables|/Game/Items/Inventory/BP_LootContainer.BP_LootContainer_C|GetItemInventory _interacted_loot_container))
  (Variables|Default|SetItemAdded item)
  (Variables|Default|SetSourceInventory (Variables|Default|GetBackpack%20Inventory))
  (Variables|Default|SetTemp%20Added%20Item%20Amount deltaValue)
  (Variables|Default|SetTemp%20Template%20ID (Variables|/Script/ConanSandbox.GameItem|GetTemplateID (Variables|Default|GetItemAdded)))
  (if (not (Default|IsAdmin (Variables|Default|GetBasePlayerChar)))
    (bind _returnvalue (Utilities|GetDataTableRow "/Game/Mods/Ash-and-Blood/DataTables/DefaultTables/DT_ItemLimitations.DT_ItemLimitations" "Potions")
      (:then
        (Variables|Default|SetTemp%20Max%20Value (.MaxValue (Utilities|Struct|BreakST_ItemAmountLimitations _returnvalue)))
        (if (Utilities|Array|ContainsItem (.ItemTemplateIDstoCheck (Utilities|Struct|BreakST_ItemAmountLimitations _returnvalue)) (Variables|Default|GetTemp%20Template%20ID))
          (bind _potions_current (CallFunction|CheckPotionCount))
          (bind _output_get (Variables|Default|SetTemp%20Potions%20Current _potions_current))
          (if (not (<= (+ _output_get (Variables|Default|GetTemp%20Added%20Item%20Amount)) (Variables|Default|GetTemp%20Max%20Value)))
            (Variables|Default|SetTemp%20Return%20Items%20to%20Source%20Inventory (- (+ (Variables|Default|GetTemp%20Potions%20Current) (Variables|Default|GetTemp%20Added%20Item%20Amount)) (Variables|Default|GetTemp%20Max%20Value)))
            (bind _output_get_2 (Variables|Default|SetTemp%20Add%20Items%20to%20Target%20Inventory (- (Class|GameItem|GetIntStat (Variables|Default|GetItemAdded) "StackSize") (- (+ (Variables|Default|GetTemp%20Potions%20Current) (Variables|Default|GetTemp%20Added%20Item%20Amount)) (Variables|Default|GetTemp%20Max%20Value)))))
            (Class|GameItem|SetIntStat (Variables|Default|GetItemAdded) "StackSize" _output_get_2 true)
            (Utilities|IsValid _interactedstoragecontainer
              (:Is%20Valid
                (Utilities|IsValid _placeableinventory
                  (:Is%20Valid
                    (Class|ItemInventory|AddItemTemplate _placeableinventory (Variables|Default|GetTemp%20Template%20ID) -1 "None" (Variables|Default|GetTemp%20Return%20Items%20to%20Source%20Inventory) false 1.0 -1.0))))
              (:Is%20Not%20Valid
                (Utilities|IsValid _interacted_loot_container
                  (:Is%20Valid
                    (Utilities|IsValid _iteminventory
                      (:Is%20Valid
                        (Class|ItemInventory|AddItemTemplate _iteminventory (Variables|Default|GetTemp%20Template%20ID) -1 "None" (Variables|Default|GetTemp%20Return%20Items%20to%20Source%20Inventory) false 1.0 -1.0)))))))))))))

(event Custom|OnItemAddedToShortcutBar
  (params (index :type Integer) (item :type Game%20Item%20Object%20Reference) (srcInventory :type Item%20Inventory%20Object%20Reference) (srcIndex :type Integer))
  (Variables|Default|SetItemAdded item)
  (Variables|Default|SetTarget%20Inventory (Variables|/Game/Characters/BasePlayerChar.BasePlayerChar_C|GetShortcutBarInventory (Variables|Default|GetBasePlayerChar)))
  (Variables|Default|SetSourceInventory srcInventory)
  (if (not (Default|IsAdmin (Variables|Default|GetBasePlayerChar)))
    (Variables|Default|SetTemp%20Template%20ID (Variables|/Script/ConanSandbox.GameItem|GetTemplateID (Variables|Default|GetItemAdded)))
    (Variables|Default|SetTemp%20Added%20Item%20Amount (Class|GameItem|GetIntStat (Variables|Default|GetItemAdded) "StackSize"))
    (bind _returnvalue (Utilities|GetDataTableRow "/Game/Mods/Ash-and-Blood/DataTables/DefaultTables/DT_ItemLimitations.DT_ItemLimitations" "Potions")
      (:then
        (Variables|Default|SetTemp%20Max%20Value (.MaxValue (Utilities|Struct|BreakST_ItemAmountLimitations _returnvalue)))
        (if (Utilities|Array|ContainsItem (.ItemTemplateIDstoCheck (Utilities|Struct|BreakST_ItemAmountLimitations _returnvalue)) (Variables|Default|GetTemp%20Template%20ID))
          (Utilities|IsValid (Variables|Default|GetSourceInventory)
            (:Is%20Valid
              (if (and (!= (Variables|Default|GetSourceInventory) (Variables|Default|GetShortcutBar%20Inventory)) (!= (Variables|Default|GetSourceInventory) (Variables|Default|GetBackpack%20Inventory)))
                (bind _potions_current (CallFunction|CheckPotionCount))
                (Variables|Default|SetTemp%20Potions%20Current _potions_current)
                (if (< (Variables|Default|GetTemp%20Potions%20Current) (Variables|Default|GetTemp%20Max%20Value))
                  (Variables|Default|SetTemp%20Add%20Items%20to%20Target%20Inventory (- (Variables|Default|GetTemp%20Max%20Value) (Variables|Default|GetTemp%20Potions%20Current)))
                  (Utilities|FlowControl|Delay 0.2)
                  (Variables|Default|SetTemp%20Return%20Items%20to%20Source%20Inventory (- (Variables|Default|GetTemp%20Added%20Item%20Amount) (Variables|Default|GetTemp%20Add%20Items%20to%20Target%20Inventory)))
                  (Class|ItemInventory|DeleteItemsbyTemplate (Variables|Default|GetTarget%20Inventory) (Variables|Default|GetTemp%20Template%20ID) "None" (- (Variables|Default|GetTemp%20Added%20Item%20Amount) (Variables|Default|GetTemp%20Add%20Items%20to%20Target%20Inventory)))
                  (if (!= (Variables|Default|GetTemp%20Return%20Items%20to%20Source%20Inventory) 0)
                    (Utilities|IsValid (Variables|Default|GetSourceInventory)
                      (:Is%20Valid
                        (Class|ItemInventory|AddItemTemplate (Variables|Default|GetSourceInventory) (Variables|Default|GetTemp%20Template%20ID) -1 "None" (Variables|Default|GetTemp%20Return%20Items%20to%20Source%20Inventory) false 1.0 -1.0))))
                  (else
                    (Utilities|IsValid (Variables|Default|GetSourceInventory)
                      (:Is%20Valid
                        (Utilities|FlowControl|Delay 0.2)
                        (Class|ItemInventory|AddItemTemplate (Variables|Default|GetSourceInventory) (Variables|Default|GetTemp%20Template%20ID) -1 "None" (Variables|Default|GetTemp%20Added%20Item%20Amount) false 1.0 -1.0)
                        (Class|ItemInventory|DeleteItemsbyTemplate (Variables|Default|GetTarget%20Inventory) (Variables|Default|GetTemp%20Template%20ID) "None" (Variables|Default|GetTemp%20Added%20Item%20Amount))))))))))))))

(event Custom|OnIntStatChangedShortcutBar
  (params (item :type Game%20Item%20Object%20Reference) (statID :type EItemIntStatID%20Enum) (statValue :type Integer) (deltaValue :type Integer))
  (bind _interactedstoragecontainer (Variables|Default|GetInteractedStorageContainer))
  (bind _interacted_loot_container (Variables|Default|GetInteracted%20Loot%20Container))
  (bind _placeableinventory (Variables|/Game/Systems/Building/Placeables/BP_PlaceableItemContainer.BP_PlaceableItemContainer_C|GetPlaceableInventory _interactedstoragecontainer))
  (bind _iteminventory (Variables|/Game/Items/Inventory/BP_LootContainer.BP_LootContainer_C|GetItemInventory _interacted_loot_container))
  (Variables|Default|SetItemAdded item)
  (Variables|Default|SetSourceInventory (Variables|Default|GetShortcutBar%20Inventory))
  (Variables|Default|SetTemp%20Added%20Item%20Amount deltaValue)
  (Variables|Default|SetTemp%20Template%20ID (Variables|/Script/ConanSandbox.GameItem|GetTemplateID (Variables|Default|GetItemAdded)))
  (if (not (Default|IsAdmin (Variables|Default|GetBasePlayerChar)))
    (bind _returnvalue (Utilities|GetDataTableRow "/Game/Mods/Ash-and-Blood/DataTables/DefaultTables/DT_ItemLimitations.DT_ItemLimitations" "Potions")
      (:then
        (Variables|Default|SetTemp%20Max%20Value (.MaxValue (Utilities|Struct|BreakST_ItemAmountLimitations _returnvalue)))
        (if (Utilities|Array|ContainsItem (.ItemTemplateIDstoCheck (Utilities|Struct|BreakST_ItemAmountLimitations _returnvalue)) (Variables|Default|GetTemp%20Template%20ID))
          (bind _potions_current (CallFunction|CheckPotionCount))
          (bind _output_get (Variables|Default|SetTemp%20Potions%20Current _potions_current))
          (if (not (<= (+ _output_get (Variables|Default|GetTemp%20Added%20Item%20Amount)) (Variables|Default|GetTemp%20Max%20Value)))
            (Variables|Default|SetTemp%20Return%20Items%20to%20Source%20Inventory (- (+ (Variables|Default|GetTemp%20Potions%20Current) (Variables|Default|GetTemp%20Added%20Item%20Amount)) (Variables|Default|GetTemp%20Max%20Value)))
            (bind _output_get_2 (Variables|Default|SetTemp%20Add%20Items%20to%20Target%20Inventory (- (Class|GameItem|GetIntStat (Variables|Default|GetItemAdded) "StackSize") (- (+ (Variables|Default|GetTemp%20Potions%20Current) (Variables|Default|GetTemp%20Added%20Item%20Amount)) (Variables|Default|GetTemp%20Max%20Value)))))
            (Class|GameItem|SetIntStat (Variables|Default|GetItemAdded) "StackSize" _output_get_2 true)
            (Utilities|IsValid _interactedstoragecontainer
              (:Is%20Valid
                (Utilities|IsValid _placeableinventory
                  (:Is%20Valid
                    (Class|ItemInventory|AddItemTemplate _placeableinventory (Variables|Default|GetTemp%20Template%20ID) -1 "None" (Variables|Default|GetTemp%20Return%20Items%20to%20Source%20Inventory) false 1.0 -1.0))))
              (:Is%20Not%20Valid
                (Utilities|IsValid _interacted_loot_container
                  (:Is%20Valid
                    (Utilities|IsValid _iteminventory
                      (:Is%20Valid
                        (Class|ItemInventory|AddItemTemplate _iteminventory (Variables|Default|GetTemp%20Template%20ID) -1 "None" (Variables|Default|GetTemp%20Return%20Items%20to%20Source%20Inventory) false 1.0 -1.0)))))))))))))

(event Custom|Custom%20Interactable%20Activate
  ;[0 1 0.06933] Custom Interactable Activate
  (bind _asfun_combat_player_controller (Utilities|Casting|CastToFunCombat_PlayerController (Pawn|GetController (Variables|Default|GetBasePlayerChar))))
  (EventDispatchers|BindEventtoOnInteractableActivate (Default|GetInteractionManager _asfun_combat_player_controller) (delegate Custom|OnInteractPressed)))

(event Custom|Server%20Set%20Interacted%20Storage%20Container
  (params (InteractedStorageContainer :type BP%20Placeable%20Item%20Container%20Object%20Reference))
  (Variables|Default|SetInteractedStorageContainer InteractedStorageContainer))

(event Custom|Server%20Set%20Interacted%20Loot%20Container
  (params (Interacted%20Loot%20Container :type BP%20Loot%20Container%20Object%20Reference))
  (Variables|Default|SetInteracted%20Loot%20Container Interacted%20Loot%20Container))

(event Custom|Server%20Set%20Interacted%20Crafting%20Station
  (params (Interacted%20Crafting%20Station :type BP%20PL%20Crafting%20Station%20Object%20Reference))
  (Variables|Default|SetInteracted%20Crafting%20Station Interacted%20Crafting%20Station))

(event Custom|CustomOnTakeAnyDamage
  (params (DamagedActor :type Actor%20Object%20Reference) (Damage :type Float%20%28single-precision%29) (DamageType :type Damage%20Type%20Object%20Reference) (InstigatedBy :type Controller%20Object%20Reference) (DamageCauser :type Actor%20Object%20Reference) (DamageEventID :type Integer))
  (bind _baseplayerchar (Variables|Default|GetBasePlayerChar))
  (bind _00_bp_ac_buffsystem (Variables|/Game/Characters/BaseBPCombat.BaseBPCombat_C|Get00_BP_AC_BuffSystem _baseplayerchar))
  (bind _hasbuff (Default|CheckifBuffExists _00_bp_ac_buffsystem "/Game/Systems/Buffs/Heal_OverTime/00_BP_AC_Buff_Vitality20aPerk_HoT.00_BP_AC_Buff_Vitality20aPerk_HoT_C"))
  (if _hasbuff
    (Default|RemoveBuff _00_bp_ac_buffsystem "/Game/Systems/Buffs/Heal_OverTime/00_BP_AC_Buff_Vitality20aPerk_HoT.00_BP_AC_Buff_Vitality20aPerk_HoT_C")
    (Class|ConanCharacter|SetIntStat (Variables|Default|GetBasePlayerChar) "HealthCurrent" (- (Class|ConanCharacter|GetIntStat (Variables|Default|GetBasePlayerChar) "HealthCurrent" "Full") (Math|Float|Truncate Damage)))
    (bind _hasbuff_2 (Default|CheckifBuffExists _00_bp_ac_buffsystem "/Game/Mods/Ash-and-Blood/BluePrints/Buffs/Custom_00_BP_AC_Buff_Vitality20aPerk_HoT.Custom_00_BP_AC_Buff_Vitality20aPerk_HoT_C"))
    (if _hasbuff_2
      (Default|RemoveBuff _00_bp_ac_buffsystem "/Game/Mods/Ash-and-Blood/BluePrints/Buffs/Custom_00_BP_AC_Buff_Vitality20aPerk_HoT.Custom_00_BP_AC_Buff_Vitality20aPerk_HoT_C"))
    (bind _newbuffwasadded (Default|AddBuff _00_bp_ac_buffsystem "/Game/Mods/Ash-and-Blood/BluePrints/Buffs/Custom_00_BP_AC_Buff_Vitality20aPerk_HoT.Custom_00_BP_AC_Buff_Vitality20aPerk_HoT_C" (Math|Float|Truncate Damage)))
    (Development|PrintString (Utilities|String|ToString(Text) (Utilities|Text|FormatText "Custom Buff Added == {bool}" (Utilities|Text|ToText(String) (Utilities|String|ToString(Boolean) _newbuffwasadded)))))))

(event Custom|OnItemAddedToBackpack
  (params (index :type Integer) (item :type Game%20Item%20Object%20Reference) (srcInventory :type Item%20Inventory%20Object%20Reference) (srcIndex :type Integer))
  (Variables|Default|SetItemAdded item)
  (Variables|Default|SetTarget%20Inventory (Variables|/Game/Characters/BasePlayerChar.BasePlayerChar_C|GetBackpackInventory (Variables|Default|GetBasePlayerChar)))
  (Variables|Default|SetSourceInventory srcInventory)
  (if (not (Default|IsAdmin (Variables|Default|GetBasePlayerChar)))
    (Variables|Default|SetTemp%20Template%20ID (Variables|/Script/ConanSandbox.GameItem|GetTemplateID (Variables|Default|GetItemAdded)))
    (Variables|Default|SetTemp%20Added%20Item%20Amount (Class|GameItem|GetIntStat (Variables|Default|GetItemAdded) "StackSize"))
    (bind _returnvalue (Utilities|GetDataTableRow "/Game/Mods/Ash-and-Blood/DataTables/DefaultTables/DT_ItemLimitations.DT_ItemLimitations" "Potions")
      (:then
        (Variables|Default|SetTemp%20Max%20Value (.MaxValue (Utilities|Struct|BreakST_ItemAmountLimitations _returnvalue)))
        (if (Utilities|Array|ContainsItem (.ItemTemplateIDstoCheck (Utilities|Struct|BreakST_ItemAmountLimitations _returnvalue)) (Variables|Default|GetTemp%20Template%20ID))
          (Utilities|IsValid (Variables|Default|GetSourceInventory)
            (:Is%20Valid
              (if (and (!= (Variables|Default|GetSourceInventory) (Variables|Default|GetShortcutBar%20Inventory)) (!= (Variables|Default|GetSourceInventory) (Variables|Default|GetBackpack%20Inventory)))
                (bind _potions_current (CallFunction|CheckPotionCount))
                (Variables|Default|SetTemp%20Potions%20Current _potions_current)
                (if (< (Variables|Default|GetTemp%20Potions%20Current) (Variables|Default|GetTemp%20Max%20Value))
                  (Variables|Default|SetTemp%20Add%20Items%20to%20Target%20Inventory (- (Variables|Default|GetTemp%20Max%20Value) (Variables|Default|GetTemp%20Potions%20Current)))
                  (Utilities|FlowControl|Delay 0.2)
                  (Variables|Default|SetTemp%20Return%20Items%20to%20Source%20Inventory (- (Variables|Default|GetTemp%20Added%20Item%20Amount) (Variables|Default|GetTemp%20Add%20Items%20to%20Target%20Inventory)))
                  (Class|ItemInventory|DeleteItemsbyTemplate (Variables|Default|GetTarget%20Inventory) (Variables|Default|GetTemp%20Template%20ID) "None" (- (Variables|Default|GetTemp%20Added%20Item%20Amount) (Variables|Default|GetTemp%20Add%20Items%20to%20Target%20Inventory)))
                  (if (!= (Variables|Default|GetTemp%20Return%20Items%20to%20Source%20Inventory) 0)
                    (Utilities|IsValid (Variables|Default|GetSourceInventory)
                      (:Is%20Valid
                        (Class|ItemInventory|AddItemTemplate (Variables|Default|GetSourceInventory) (Variables|Default|GetTemp%20Template%20ID) -1 "None" (Variables|Default|GetTemp%20Return%20Items%20to%20Source%20Inventory) false 1.0 -1.0))))
                  (else
                    (Utilities|IsValid (Variables|Default|GetSourceInventory)
                      (:Is%20Valid
                        (Utilities|FlowControl|Delay 0.2)
                        (Class|ItemInventory|AddItemTemplate (Variables|Default|GetSourceInventory) (Variables|Default|GetTemp%20Template%20ID) -1 "None" (Variables|Default|GetTemp%20Added%20Item%20Amount) false 1.0 -1.0)
                        (Class|ItemInventory|DeleteItemsbyTemplate (Variables|Default|GetTarget%20Inventory) (Variables|Default|GetTemp%20Template%20ID) "None" (Variables|Default|GetTemp%20Added%20Item%20Amount))))))))))))))

(event Custom|Restrict%20Specific%20Items%20by%20Amount%20OnItemAdded
  (bind _baseplayerchar (Variables|Default|GetBasePlayerChar))
  (Variables|Default|SetBackpack%20Inventory (Variables|/Game/Characters/BasePlayerChar.BasePlayerChar_C|GetBackpackInventory _baseplayerchar))
  (Variables|Default|SetShortcutBar%20Inventory (Variables|/Game/Characters/BasePlayerChar.BasePlayerChar_C|GetShortcutBarInventory _baseplayerchar))
  (EventDispatchers|BindEventtoSignalItemAdded (Variables|Default|GetBackpack%20Inventory) (delegate Custom|OnItemAddedToBackpack))
  (EventDispatchers|BindEventtoSignalItemAdded (Variables|Default|GetShortcutBar%20Inventory) (delegate Custom|OnItemAddedToShortcutBar))
  (CallFunction|RestrictSpecificItemsbyAmountIntStatChange))

(event Custom|Calculate%20Storage%20Used
  (bind _modcontroller (Variables|Default|GetModController))
  (bind _baseplayerchar (Variables|Default|GetBasePlayerChar))
  (Variables|Default|SetStorage%20Used 0)
  (Variables|Default|SetBonus%20Building%20Pieces 0)
  (Variables|Default|SetBonus%20Placeable%20Pieces 0)
  (Variables|Default|SetBonus%20Storage%20Capacity 0)
  (bind _returnvalue (Class|ConanWorldSettings|GetPlayerPawnRegistry (Class|FuncomGenericLibrary|GetWorldSettings)))
  (bind _returnvalue_2 (Class|PlayerPawnRegistry|GetPlayerPawns _returnvalue))
  (for _array_element _returnvalue_2
    (bind _asbase_player_char (Utilities|Casting|CastToBasePlayerChar _array_element))
    (if (== _asbase_player_char _baseplayerchar)
      (Variables|Default|SetHas%20Role%20Index -1 :!label _label)
      (for (_array_element_2 _array_index) (Variables|/Game/Mods/Ash-and-Blood/MC_AnB.MC_AnB_C|GetLimit%20-%20Sudo%20Role (Variables|Default|GetModController))
        (bind _has_role (Class|IEAACPlayerAuth|HasRole(Message) (Class|Actor|GetComponentbyInterface _asbase_player_char "/Game/ModsShared/SudoExile/Auth/I_EA_AC_Player_Auth.I_EA_AC_Player_Auth_C") (Utilities|String|StringToName _array_element_2)))
        (if _has_role
          (if (Utilities|Enum|Equal(Enum) _array_element_2 "Mod")
            (Variables|Default|SetHas%20Role%20Index _array_index)
            (else
              (Variables|Default|SetBonus%20Building%20Pieces 250)
              (Variables|Default|SetBonus%20Placeable%20Pieces 150)
              (Variables|Default|SetBonus%20Storage%20Capacity 150)))))
      (if (!= (Variables|Default|GetHas%20Role%20Index) -1)
        (Variables|Default|SetBonus%20Building%20Pieces (+ (Variables|Default|GetBonus%20Building%20Pieces) (Utilities|Array|Get(acopy) (Variables|/Game/Mods/Ash-and-Blood/MC_AnB.MC_AnB_C|GetLimit%20-%20Sudo%20Role%20Build%20Piece%20Bonus _modcontroller) (Variables|Default|GetHas%20Role%20Index))))
        (Variables|Default|SetBonus%20Placeable%20Pieces (+ (Variables|Default|GetBonus%20Placeable%20Pieces) (Utilities|Array|Get(acopy) (Variables|/Game/Mods/Ash-and-Blood/MC_AnB.MC_AnB_C|GetLimit%20-%20Sudo%20Role%20Placeable%20Piece%20Bonus _modcontroller) (Variables|Default|GetHas%20Role%20Index))))
        (Variables|Default|SetBonus%20Storage%20Capacity (+ (Variables|Default|GetBonus%20Storage%20Capacity) (Utilities|Array|Get(acopy) (Variables|/Game/Mods/Ash-and-Blood/MC_AnB.MC_AnB_C|GetLimit%20-%20Sudo%20Role%20Storage%20Bonus _modcontroller) (Variables|Default|GetHas%20Role%20Index)))))
      (elif (Default|IsinSameGuild _asbase_player_char _baseplayerchar)
        (goto _label))))
  (bind _outactors (Actor|GetAllActorsOfClass "/Game/Systems/Building/Placeables/BP_PlaceableItemContainer.BP_PlaceableItemContainer_C"))
  (for _array_element_3 _outactors
    (if (Class|BuildableBase|IsOwner _array_element_3 (Variables|Default|GetBasePlayerChar) false)
      (Utilities|GetDataTableRow "/Game/Mods/Ash-and-Blood/DataTables/DefaultTables/DT_StorageLimitationsExceptions.DT_StorageLimitationsExceptions" (Utilities|String|StringToName (Utilities|String|ToString(Integer) (Variables|/Script/ConanSandbox.BuildableBase|GetTemplateId _array_element_3)))
        (:RowNotFound
          (bind _returnvalue_3 (Utilities|GetDataTableRow "/Game/Mods/Ash-and-Blood/DataTables/DefaultTables/DT_StorageLimitations.DT_StorageLimitations" (Utilities|String|StringToName (Utilities|String|ToString(Integer) (Variables|/Script/ConanSandbox.BuildableBase|GetTemplateId _array_element_3))))
            (:then
              (Variables|Default|SetStorage%20Used (+ (Variables|Default|GetStorage%20Used) (Utilities|Struct|BreakST_StorageLimitations _returnvalue_3)))))))))
  (Variables|Default|SetUpdate%20Guild%20UI (select (Variables|Default|GetUpdate%20Guild%20UI) false true)))

(event Custom|Server%20Set%20Active%20Thrall%20Bonuses
  (params (Crafting%20Station :type BP%20PL%20Crafting%20Station%20Object%20Reference) (Active%20Thrall :type Name) (New%20Active%20Thrall%20Bonus%20Row :type Name) (Thrall%20Profession :type Name))
  (Default|UpdateBonusRecipeLIst (Actor|GetComponentbyClass Crafting%20Station "/Game/Mods/Ash-and-Blood/BluePrints/ActorComponents/AC_CustomCraftingSystem.AC_CustomCraftingSystem_C") Active%20Thrall New%20Active%20Thrall%20Bonus%20Row Thrall%20Profession))

(fn OnRepUpdateGuildUI
  (if (not (Networking|IsServer))
    (bind _foundwidgets (Widget|GetAllWidgetsOfClass "/Game/Mods/Ash-and-Blood/UserInterface/W_AAB_GuildView.W_AAB_GuildView_C" true))
    (Default|SetStorageCapacityUsed (Utilities|Array|Get(acopy) _foundwidgets) (Variables|Default|GetStorage%20Used) (Variables|Default|GetBonus%20Building%20Pieces) (Variables|Default|GetBonus%20Placeable%20Pieces) (Variables|Default|GetBonus%20Storage%20Capacity))))

(fn CheckPotionCount
  (bind _baseplayerchar (Variables|Default|GetBasePlayerChar))
  (Variables|Default|SetTemp%20Potions%20Current 0)
  (for _array_element (Variables|/Script/ConanSandbox.ItemInventory|GetItemList (Variables|/Game/Characters/BasePlayerChar.BasePlayerChar_C|GetBackpackInventory _baseplayerchar))
    (if (Utilities|IsValid _array_element)
      (bind _returnvalue (Utilities|GetDataTableRow "/Game/Mods/Ash-and-Blood/DataTables/DefaultTables/DT_ItemLimitations.DT_ItemLimitations" "Potions")
        (:then
          (LocalVariables|SetLOC%20Max%20Value (.MaxValue (Utilities|Struct|BreakST_ItemAmountLimitations _returnvalue)))
          (if (Utilities|Array|ContainsItem (.ItemTemplateIDstoCheck (Utilities|Struct|BreakST_ItemAmountLimitations _returnvalue)) (Variables|/Script/ConanSandbox.GameItem|GetTemplateID _array_element))
            (Variables|Default|SetTemp%20Potions%20Current (+ (Variables|Default|GetTemp%20Potions%20Current) (Class|GameItem|GetIntStat _array_element "StackSize"))))))))
  (for _array_element_2 (Variables|/Script/ConanSandbox.ItemInventory|GetItemList (Variables|/Game/Characters/BasePlayerChar.BasePlayerChar_C|GetShortcutBarInventory _baseplayerchar))
    (if (Utilities|IsValid _array_element_2)
      (bind _returnvalue_2 (Utilities|GetDataTableRow "/Game/Mods/Ash-and-Blood/DataTables/DefaultTables/DT_ItemLimitations.DT_ItemLimitations" "Potions")
        (:then
          (LocalVariables|SetLOC%20Max%20Value (.MaxValue (Utilities|Struct|BreakST_ItemAmountLimitations _returnvalue_2)))
          (if (Utilities|Array|ContainsItem (.ItemTemplateIDstoCheck (Utilities|Struct|BreakST_ItemAmountLimitations _returnvalue_2)) (Variables|/Script/ConanSandbox.GameItem|GetTemplateID _array_element_2))
            (Variables|Default|SetTemp%20Potions%20Current (+ (Variables|Default|GetTemp%20Potions%20Current) (Class|GameItem|GetIntStat _array_element_2 "StackSize"))))))))
  (return (- (Variables|Default|GetTemp%20Potions%20Current) (Variables|Default|GetTemp%20Added%20Item%20Amount))))
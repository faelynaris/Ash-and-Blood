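; Preview-style actor in the rune system that displays a swappable static or skeletal mesh and lets it be rotated by mouse drag.
; Setting a mesh resets rotation, then uniformly rescales it to fit within DesireExtend and offsets it to center its bounds.
; Click start and end toggle rotation, while mouse-over applies the cursor delta as yaw and pitch to the parent Scene component.
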(event Custom|UpdateScale
  (bind _desireextend (Variables|Default|GetDesireExtend))
  (bind _staticmesh (Variables|Default|GetStaticMesh))
  (Variables|Default|SetCurrentExtendMesh (.BoxExtent (Collision|GetComponentBounds (Variables|Default|GetStaticMesh))))
  (Transformation|SetWorldScale3D _staticmesh (* (Transformation|GetWorldScale _staticmesh) (Math|Float|Min(Float) (/ (.x _desireextend) (.x (Variables|Default|GetCurrentExtendMesh))) (/ (.y _desireextend) (.y (Variables|Default|GetCurrentExtendMesh))) (/ (.z _desireextend) (.z (Variables|Default|GetCurrentExtendMesh))))))
  (Transformation|AddLocalOffset (Variables|Default|GetStaticMesh) (- (Transformation|GetWorldLocation _staticmesh) (.Origin (Collision|GetComponentBounds _staticmesh))) false true))

(event Custom|OnClickEnd
  (params (Mouse%20Location :type Vector%202D%20Structure))
  (Variables|Default|SetRotationEnabled false))

(event Custom|OnMouseOver
  (params (Mouse%20Location :type Vector%202D%20Structure))
  (if (Variables|Default|GetRotationEnabled)
    (Transformation|AddWorldRotation (Variables|Default|GetScene) (Math|Rotator|MakeRotator 0.0 (.Y (Math|Vector2D|BreakVector2D (- Mouse%20Location (Variables|Default|GetOnStartRotation)))) (* (.X (Math|Vector2D|BreakVector2D (- Mouse%20Location (Variables|Default|GetOnStartRotation)))) -1.0)) false false)
    (Variables|Default|SetOnStartRotation Mouse%20Location)))

(event Custom|UpdateScaleSK
  (bind _desireextend (Variables|Default|GetDesireExtend))
  (bind _skeletalmesh (Variables|Default|GetSkeletalMesh))
  (Variables|Default|SetCurrentExtendMesh (.BoxExtent (Collision|GetComponentBounds (Variables|Default|GetSkeletalMesh))))
  (Transformation|SetWorldScale3D (Variables|Default|GetSkeletalMesh) (* (Transformation|GetWorldScale (Variables|Default|GetSkeletalMesh)) (Math|Float|Min(Float) (/ (.x _desireextend) (.x (Variables|Default|GetCurrentExtendMesh))) (/ (.y _desireextend) (.y (Variables|Default|GetCurrentExtendMesh))) (/ (.z _desireextend) (.z (Variables|Default|GetCurrentExtendMesh))))))
  (Transformation|AddLocalOffset (Variables|Default|GetSkeletalMesh) (- (Transformation|GetWorldLocation _skeletalmesh) (.Origin (Collision|GetComponentBounds _skeletalmesh))) false false))

(event Custom|OnClickStart
  (params (Mouse%20Location :type Vector%202D%20Structure))
  (Variables|Default|SetOnStartRotation Mouse%20Location)
  (Variables|Default|SetRotationEnabled true))

(fn ConstructionScript)

(fn SetNewMash
  (params (Mesh :type Static%20Mesh%20Object%20Reference))
  (bind _staticmesh (Variables|Default|GetStaticMesh))
  (Components|StaticMesh|SetStaticMesh _staticmesh Mesh)
  (Transformation|SetRelativeRotation _staticmesh "0, 0, 0" false true)
  (Transformation|SetRelativeRotation (Variables|Default|GetScene) "0, 0, 0" false false)
  (CallFunction|UpdateScale))

(fn SetNewMashSK
  (params (Skeletal%20Mesh :type Skeletal%20Mesh%20Object%20Reference))
  (bind _skeletalmesh (Variables|Default|GetSkeletalMesh))
  (Class|SkinnedMeshComponent|SetSkeletalMesh _skeletalmesh Skeletal%20Mesh true)
  (Transformation|SetRelativeRotation _skeletalmesh "0, 0, 0" false true)
  (Transformation|SetRelativeRotation (Variables|Default|GetScene) "0, 0, 0" false false)
  (CallFunction|UpdateScaleSK))
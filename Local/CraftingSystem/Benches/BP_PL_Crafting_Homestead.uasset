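; Homestead crafting bench placeable that supports thralls and exposes an artisan thrall inventory.
; Unless it is a brush, it listens to its cook work slot's state changes, applying the current state on BeginPlay and unbinding on EndPlay.
; An in-use slot hides props and turns lights on.
; Deactivated, available or reserved states show props and light the bench only while the crafting queue runs.
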(event Custom|SlotStateChanged
  (params (SlotComponent :type Smart%20Object%20Slot%20Component%20Object%20Reference) (PrevState :type ESmartObjectSlotState%20Enum) (NewState :type ESmartObjectSlotState%20Enum))
  (bind _bp_bac_turnlightonoff (Variables|Default|GetBP_BAC_TurnLightOnOff))
  (switch Utilities|FlowControl|Switch|SwitchonESmartObjectSlotState NewState
    (:Deactivated
      (CallFunction|TogglePropVisibility true :!label _label)
      (if (Class|CraftingQueue|IsRunning (Variables|Default|GetCraftingQueue))
        (Default|TurnonAll _bp_bac_turnlightonoff)
        (else
          (Default|TurnOffAll _bp_bac_turnlightonoff))))
    (:Available
      (goto _label))
    (:Reserved
      (goto _label))
    (:InUse
      (CallFunction|TogglePropVisibility false)
      (Default|TurnonAll (Variables|Default|GetBP_BAC_TurnLightOnOff)))))

(event EventEndPlay
  (params (EndPlayReason :type EEndPlayReason%20Enum :default "Destroyed"))
  (|CallParentFunction EndPlayReason)
  (EventDispatchers|UnbindallEventsfromOnStateChanged (Variables|Default|GetSOS_Work_Cook)))

(event EventBeginPlay
  (if (not (Class|CraftingQueue|IsRunning (Variables|Default|GetCraftingQueue)))
    (Default|TurnOffAll (Variables|Default|GetBP_BAC_TurnLightOnOff)))
  (|CallParentFunction)
  (if (not (Variables|Default|GetIsABrush))
    (EventDispatchers|BindEventtoOnStateChanged (Variables|Default|GetSOS_Work_Cook) (delegate Custom|SlotStateChanged))
    (CallFunction|SlotStateChanged 0 "Deactivated" (Class|SmartObjectSlotComponent|GetState (Variables|Default|GetSOS_Work_Cook)))))

(fn ConstructionScript
  (|CallParentFunction))

(fn GetArtisanThrallInventory
  (return (Variables|Default|GetArtisanThrallInventory)))

(fn CanStationUseThralls
  (return true))